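; BP_Equip is an equippable pickup actor that the third-person character equips by overlapping its box.
; Equip checks remaining EquipLoad on the character's CT attribute component against the item's Weight, then adds the item to inventory and attaches it to a mesh socket.
; It hides the weight text, disables box collision, and applies its Weight and attribute map as load and equipment bonuses.
; Destroying the actor reverses the load and attribute changes through UnEquip.
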(event OnComponentBeginOverlap(Box)
  (params (OverlappedComponent :type Primitive%20Component%20Object%20Reference) (OtherActor :type Actor%20Object%20Reference) (OtherComp :type Primitive%20Component%20Object%20Reference) (OtherBodyIndex :type Integer) (bFromSweep :type Boolean) (SweepResult :type Hit%20Result%20Structure%20%28by%20ref%29))
  (CallFunction|Equip OtherActor (Variables|Default|GetItem)))

(event Custom|ActorUsed
  (Rendering|SetVisibility (Variables|Default|GetTextRender) false false)
  (Collision|SetCollisionEnabled (Variables|Default|GetBox) "NoCollision"))

(event EventDestroyed
  (CallFunction|UnEquip))

(fn ConstructionScript)

(fn CheckEquipLoad
  (return (>= (- (Default|GetAttribute (Variables|Default|GetCT_Cmpt_Attribute) "(TagName=\"CT.Attribute.Dynamic.EquipLoad\")") (Default|GetVariable (Variables|Default|GetCT_Cmpt_Attribute) "(TagName=\"CT.Attribute.Dynamic.EquipLoad\")")) (Variables|Default|GetWeight))))

(fn Equip
  (params (Actor :type Actor%20Object%20Reference) (String :type String))
  (Utilities|FlowControl|Sequence
    (:then_0
      (bind _asbp_third_person_character (Utilities|Casting|CastToBP_ThirdPersonCharacter Actor))
      (bind _output_get (LocalVariables|SetLocal_Character _asbp_third_person_character))
      (bind _output_get_2 (Variables|Default|SetCT_Cmpt_Attribute (Actor|GetComponentbyClass _output_get "/Game/CT_Components/AttributeSystem/Components/CT_Cmpt_Attribute.CT_Cmpt_Attribute_C")))
      (Utilities|IsValid _output_get_2
        (:Is%20Valid
          (if (not (CallFunction|CheckEquipLoad))
            (return)))
        (:Is%20Not%20Valid
          (return))))
    (:then_1
      (Default|AddItem (Variables|/Game/SpellSystemV2/SpellSystem/Blueprints/BP_ThirdPersonCharacter.BP_ThirdPersonCharacter_C|GetCT_ComponentInventory _asbp_third_person_character) String)
      (Transformation|AttachComponentToComponent (Variables|/Script/Engine.Character|GetMesh (LocalVariables|GetLocal_Character)) (Variables|Default|GetSocketName) "SnapToTarget" "SnapToTarget" "KeepRelative" true)
      (CallFunction|ActorUsed)
      (Default|IncVariable (Variables|Default|GetCT_Cmpt_Attribute) "(TagName=\"CT.Attribute.Dynamic.EquipLoad\")" (Variables|Default|GetWeight))
      (bind _keys (Utilities|Map|Keys (Variables|Default|GetAttributes)))
      (for _array_element _keys
        (Default|IncEquipAttribute (Variables|Default|GetCT_Cmpt_Attribute) _array_element (.Value (Utilities|Map|Find (Variables|Default|GetAttributes) _array_element)))))))

(fn UnEquip
  (Utilities|IsValid (Variables|Default|GetCT_Cmpt_Attribute)
    (:Is%20Valid
      (Default|IncVariable (Variables|Default|GetCT_Cmpt_Attribute) "(TagName=\"CT.Attribute.Dynamic.EquipLoad\")" (* (Variables|Default|GetWeight) -1.0))
      (bind _keys (Utilities|Map|Keys (Variables|Default|GetAttributes)))
      (for _array_element _keys
        (Default|IncEquipAttribute (Variables|Default|GetCT_Cmpt_Attribute) _array_element (* (.Value (Utilities|Map|Find (Variables|Default|GetAttributes) _array_element)) -1.0))))))

(fn PickUpItem
  (return ""))