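; BP_PoolTest is a test actor that produces an experience pickup just above itself, either from a pool or by spawning it.
; The Start event's Condition picks between requesting one from BP_PoolManager via GetActorFromPool and spawning and initializing a fresh BP_EXP.
; Both paths pass the Instigator and set the pickup's speed slightly above that instigator's max walk speed.
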(event Custom|Start
  (params (Condition :type Boolean) (Instigator :type Pawn%20Object%20Reference))
  (bind _returnvalue (Actor|GetComponentbyClass Instigator "/Script/Engine.CharacterMovementComponent"))
  (bind _maxwalkspeed (Variables|/Script/Engine.CharacterMovementComponent|GetMaxWalkSpeed _returnvalue))
  (bind _returnvalue_2 (+ _maxwalkspeed 1e+02))
  ;[0 0 0] Spawn or Get From Pool - Experience
  (if Condition
    (bind _returnvalue_3 (Actor|GetActorOfClass "/Game/SpellSystemV2/LevelingSystemX/Blueprints/Actors/BP_PoolManager.BP_PoolManager_C"))
    (Default|GetActorfromPool _returnvalue_3 (Utilities|Struct|MakeS_PoolExperience (CallFunction|ExperienceSpawnLocation) Instigator 1 1 _returnvalue_2 true))
    (else
      (bind _returnvalue_4 (Game|SpawnActorfromClass "/Game/SpellSystemV2/LevelingSystemX/Blueprints/Actors/BP_EXP.BP_EXP_C" (Math|Transform|MakeTransform (CallFunction|ExperienceSpawnLocation) "0, 0, 0" "1.000000,1.000000,1.000000") "Undefined" 0 1 _returnvalue_2 2 true Instigator))
      (Default|Initialize _returnvalue_4))))

(fn ConstructionScript)

(fn ExperienceSpawnLocation
  (return (+ (Transformation|GetActorLocation) "0.000000,0.000000,25.000000")))