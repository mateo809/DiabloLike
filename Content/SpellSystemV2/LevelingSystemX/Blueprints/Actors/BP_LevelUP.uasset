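; BP_LevelUP is a self-destroying visual effect actor, apparently for level-ups, combining a decal and a Niagara effect.
; On BeginPlay, one timeline scales the decal in Y and Z while another drives the Opacity parameter of its dynamic material.
; After a short timer, Niagara deactivates and the opacity timeline reverses.
; A Forward flag lets the same Finished pin either start that timer or destroy the actor after a delay.
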(event Custom|CustomEvent
  ;[0 0 0] Begin play / Timer / Material Values
  (Components|Activation|Deactivate (Variables|Default|GetNiagara))
  (Variables|Default|SetForward false)
  (bind _time (Timeline|Timeline Reverse)
    (:Update
      (Rendering|Material|SetScalarParameterValue (stale EventBeginPlay _returnvalue) "Opacity" _time :!class /Script/Engine.MaterialInstanceDynamic))
    (:Finished
      (if (Variables|Default|GetForward)
        (Utilities|Time|SetTimerbyEvent (delegate Custom|CustomEvent) 0.2)
        (else
          (Utilities|FlowControl|Delay 0.5)
          (Actor|DestroyActor))))))

(event EventBeginPlay
  ;[0 0 0] Begin play / Timer / Material Values
  (bind _returnvalue (Rendering|Material|CreateDynamicMaterialInstance (Variables|Default|GetDecal) :!class /Script/Engine.DecalComponent))
  (Utilities|FlowControl|Sequence
    (:then_0
      (bind _time (Timeline|Timeline_0 Play)
        (:Update
          (Transformation|SetRelativeScale3D (Variables|Default|GetDecal) (Math|Vector|MakeVector 1.0 _time _time)))))
    (:then_1
      (bind _time_2 (Timeline|Timeline Play)
        (:Update
          (Rendering|Material|SetScalarParameterValue _returnvalue "Opacity" _time_2 :!class /Script/Engine.MaterialInstanceDynamic))
        (:Finished
          (if (Variables|Default|GetForward)
            (Utilities|Time|SetTimerbyEvent (delegate Custom|CustomEvent) 0.2)
            (else
              (Utilities|FlowControl|Delay 0.5)
              (Actor|DestroyActor))))))))

(fn ConstructionScript)