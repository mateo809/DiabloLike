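; Test trigger for the pooling system that starts every BP_PoolTest actor in the level, with pooling on or off.
; Its text label shows green ON or red OFF from the Pool flag at BeginPlay.
; A character overlapping the cube opens a gate and, after a short delay, repeatedly calls Start on those actors, passing Pool and the character.
; Any end overlap closes the gate, blocking a pending trigger.
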(event OnComponentBeginOverlap(Cube)
  (params (OverlappedComponent :type Primitive%20Component%20Object%20Reference) (OtherActor :type Actor%20Object%20Reference) (OtherComp :type Primitive%20Component%20Object%20Reference) (OtherBodyIndex :type Integer) (bFromSweep :type Boolean) (SweepResult :type Hit%20Result%20Structure%20%28by%20ref%29))
  ;[0 0 0] Overlap
  (bind _ascharacter (Utilities|Casting|CastToCharacter OtherActor))
  (Utilities|FlowControl|Sequence
    (:then_0
      (Utilities|FlowControl|Delay 0.2)
      (Utilities|FlowControl|Gate true :!label _label
        (:Exit
          (for _index (range 0 (Variables|Default|GetEXP%20-%20Actors%20%28for%20each%20actor%29))
            (bind _outactors (Actor|GetAllActorsOfClass "/Game/SpellSystemV2/LevelingSystemX/Blueprints/Actors/BP_PoolTest.BP_PoolTest_C"))
            (Default|Start _outactors (Variables|Default|GetPool) _ascharacter)))))
    (:then_1
      (goto _label Open))))

(event OnComponentEndOverlap(Cube)
  (params (OverlappedComponent :type Primitive%20Component%20Object%20Reference) (OtherActor :type Actor%20Object%20Reference) (OtherComp :type Primitive%20Component%20Object%20Reference) (OtherBodyIndex :type Integer))
  ;[0 0 0] Overlap
  (Utilities|FlowControl|Gate true) ; enters at Close
)

(event EventBeginPlay
  (bind _textrender1 (Variables|Default|GetTextRender1))
  (bind _pool (Variables|Default|GetPool))
  ;[0 0 0] Begin Play
  (Rendering|Components|TextRender|SetTextRenderColor _textrender1 (select _pool (Class|KismetMathLibrary|LinearColortoRGBE "(R=0.088719,G=1.000000,B=0.000000,A=1.000000)") (Class|KismetMathLibrary|LinearColortoRGBE "(R=1.000000,G=0.000000,B=0.000000,A=1.000000)")))
  (Rendering|Components|TextRender|SetText _textrender1 (select _pool (Utilities|Text|MakeLiteralText "ON") (Utilities|Text|MakeLiteralText "OFF"))))

(fn ConstructionScript)