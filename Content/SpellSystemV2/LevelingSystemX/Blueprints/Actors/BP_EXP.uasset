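; BP_EXP is an experience orb that flies to its instigating player, initialized either from a pool or as a spawned actor.
; Tick eases it upward, then enables homing on the player's capsule, with timed random gravity varying non-linear paths on authority.
; On overlap it triggers a level-colored Niagara effect, awards experience server-side if CollisionWithExperience is set, then returns to the pool or destroys itself.
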(event OnComponentBeginOverlap(Sphere)
  (params (OverlappedComponent :type Primitive%20Component%20Object%20Reference) (OtherActor :type Actor%20Object%20Reference) (OtherComp :type Primitive%20Component%20Object%20Reference) (OtherBodyIndex :type Integer) (bFromSweep :type Boolean) (SweepResult :type Hit%20Result%20Structure%20%28by%20ref%29))
  ;[0 0 0] Hit
  (if (Networking|IsServer)
    (CallFunction|SphereBeginOverlap(Server) OtherActor)
    (elif (== OtherActor (Game|GetInstigator))
      (Default|SpawnNiagara (Variables|Default|GetLevelingComp) (Variables|Don'tEdit|GetColor))
      (if (Variables|Don'tEdit|GetPool)
        (Default|ReturnActortoPool (Variables|Don'tEdit|GetPool%20Manager) self)
        (else
          (Actor|DestroyActor))))))

(event Custom|CustomEvent
  ;[0 0 0] Tick
  (Variables|/Script/Engine.ProjectileMovementComponent|SetProjectileGravityScale (Variables|Default|GetProjectileMovement) (Math|Random|RandomFloatinRange (Variables|Default|GetMin%20Gravity) (Variables|Default|GetMax%20Gravity))))

(event Custom|Initialize
  ;[0 0 0] Begin Play
  ;;[0 0 0] Spawned EXP - Initialize
  (Variables|Don'tEdit|SetPool false)
  (Variables|Default|SetLevelingComp (Actor|GetComponentbyClass (Game|GetInstigator) "/Game/SpellSystemV2/LevelingSystemX/Blueprints/Components/BP_Player_LevelingSystemX.BP_Player_LevelingSystemX_C"))
  (bind _color (Default|ExperienceColor (Variables|Default|GetLevelingComp) (Variables|Don'tEdit|GetLevel)))
  (bind _output_get (Variables|Don'tEdit|SetColor _color))
  (Niagara|SetNiagaraVariable(LinearColor) (Variables|Default|GetNiagara) "EXP Color User" _output_get)
  (Variables|Don'tEdit|SetTarget%20Z%20Location (+ (.z (Transformation|GetActorLocation)) 111.0))
  (Variables|Default|SetCapsule (Actor|GetComponentbyClass (Game|GetInstigator) "/Script/Engine.CapsuleComponent"))
  (Actor|Tick|SetActorTickEnabled true))

(event Custom|Sphere%20Begin%20Overlap%20%28Server%29
  (params (Actor :type Actor%20Object%20Reference))
  ;[0 0 0] Only If BP_EXP is on Server side
  (if (== Actor (Game|GetInstigator))
    (if (Variables|Don'tEdit|GetCollision%20With%20Experience)
      (Default|SpawnNiagara (Variables|Default|GetLevelingComp) (Variables|Don'tEdit|GetColor))
      (Default|AddExperience-Server (Variables|Default|GetLevelingComp) (Variables|Don'tEdit|GetExperience) (Variables|Don'tEdit|GetLevel))
      (else
        (Default|SpawnNiagara (Variables|Default|GetLevelingComp) (Variables|Don'tEdit|GetColor))))
    (if (Variables|Don'tEdit|GetPool)
      (Default|ReturnActortoPool (Variables|Don'tEdit|GetPool%20Manager) self)
      (else
        (Actor|DestroyActor)))))

(event EventInitializeExp
  (params (Experience%20Data :type S%20Pool%20Experience%20Structure) (PoolManager :type BP%20Pool%20Manager%20Object%20Reference))
  ;[0 0 0] Begin Play
  ;;[0 0 0] EXP from Pool
  (bind _output_get (Variables|Default|SetExperience%20Data Experience%20Data))
  (Variables|Actor|SetInstigator (.Instigator (Utilities|Struct|BreakS_PoolExperience _output_get)))
  (Variables|Don'tEdit|SetPool%20Manager PoolManager)
  (Variables|Don'tEdit|SetExperience (.Experience (Utilities|Struct|BreakS_PoolExperience _output_get)))
  (Variables|Don'tEdit|SetLevel (.RewardLevel (Utilities|Struct|BreakS_PoolExperience _output_get)))
  (Variables|Don'tEdit|SetCollision%20With%20Experience (.CollisionExperience (Utilities|Struct|BreakS_PoolExperience _output_get)))
  (Variables|Don'tEdit|SetSpeed (Utilities|Struct|BreakS_PoolExperience (Variables|Default|GetExperience%20Data)))
  (Variables|Don'tEdit|SetCollision%20With%20Experience (Utilities|Struct|BreakS_PoolExperience (Variables|Default|GetExperience%20Data)))
  (Variables|Don'tEdit|SetPool true)
  (Transformation|SetActorLocation (Utilities|Struct|BreakS_PoolExperience (Variables|Default|GetExperience%20Data)) false false)
  (Variables|Default|SetLevelingComp (Actor|GetComponentbyClass (Utilities|Struct|BreakS_PoolExperience (Variables|Default|GetExperience%20Data)) "/Game/SpellSystemV2/LevelingSystemX/Blueprints/Components/BP_Player_LevelingSystemX.BP_Player_LevelingSystemX_C"))
  (Default|RemovePendingExp (Variables|Don'tEdit|GetPool%20Manager) (Variables|Default|GetExperience%20Data))
  (bind _color (Default|ExperienceColor (Variables|Default|GetLevelingComp) (Variables|Don'tEdit|GetLevel)))
  (bind _output_get_2 (Variables|Don'tEdit|SetColor _color))
  (Niagara|SetNiagaraVariable(LinearColor) (Variables|Default|GetNiagara) "EXP Color User" _output_get_2)
  (Variables|Don'tEdit|SetTarget%20Z%20Location (+ (.z (Transformation|GetActorLocation)) 111.0))
  (Variables|Default|SetCapsule (Actor|GetComponentbyClass (Game|GetInstigator) "/Script/Engine.CapsuleComponent"))
  (Actor|Tick|SetActorTickEnabled true))

(event EventTick
  (params (DeltaSeconds :type Float%20%28single-precision%29))
  (bind _returnvalue (Transformation|GetActorLocation))
  (bind _target_z_location (Variables|Don'tEdit|GetTarget%20Z%20Location))
  (bind _snapping_on_the_xy_axis (Variables|Default|GetSnapping%20on%20the%20XY%20axis))
  (bind _returnvalue_2 (Math|Float|Lerp (.z _returnvalue) _target_z_location 0.1))
  ;[0 0 0] Tick
  (Transformation|SetActorLocation (Math|Vector|MakeVector (Math|Float|SelectFloat (.x _returnvalue) (Math|Float|Lerp (.x _returnvalue) (+ (.x _returnvalue) _snapping_on_the_xy_axis) 0.1) (Variables|Default|GetLinear%20Tracking)) (Math|Float|SelectFloat (.y _returnvalue) (Math|Float|Lerp (.y _returnvalue) (+ (.y _returnvalue) _snapping_on_the_xy_axis) 0.1) (Variables|Default|GetLinear%20Tracking)) _returnvalue_2) false false)
  (if (Math|Float|NearlyEqual(Float) _returnvalue_2 (Variables|Don'tEdit|GetTarget%20Z%20Location) 1.0)
    (Actor|Tick|SetActorTickEnabled false)
    (Collision|SetCollisionEnabled (Variables|Default|GetSphere) "QueryOnly")
    (Variables|/Script/Engine.ProjectileMovementComponent|SetMaxSpeed (Variables|Default|GetProjectileMovement) (Variables|Don'tEdit|GetSpeed))
    (Variables|/Script/Engine.ProjectileMovementComponent|SetHomingTargetComponent (Variables|Default|GetProjectileMovement) (Variables|Default|GetCapsule))
    (Collision|SetCollisionResponsetoChannel (Variables|Default|GetSphere) "ECC_Pawn" "ECR_Overlap")
    (Networking|SwitchHasAuthority
      (:Authority
        (if (not (Variables|Default|GetLinear%20Tracking))
          (if (Class|Actor|IsActorTickEnabled self) :!label _label
            (Utilities|FlowControl|Delay 0.1)
            (goto _label)
            (else
              (bind _returnvalue_3 (Utilities|Time|SetTimerbyEvent (delegate Custom|CustomEvent) 1.0 true -0.9))
              (Variables|Default|SetTimer _returnvalue_3))))))))

(fn ConstructionScript)

(fn OnRepColor
  (Niagara|SetNiagaraVariable(LinearColor) (Variables|Default|GetNiagara) "EXP Color User" (Variables|Don'tEdit|GetColor)))