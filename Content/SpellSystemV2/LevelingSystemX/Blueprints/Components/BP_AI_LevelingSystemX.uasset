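; AI enemy component for the leveling system that tracks health and rewards players for damage dealt.
; Hits log clamped damage per player and award rank points; lethal damage triggers ragdoll and collision changes.
; After a delay, experience is split by damage share, granted directly or through pooled or spawned BP_EXP visuals, optionally collected by collision.
; A looping timer then fades dynamic body materials before destroying the character.
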(event Custom|CustomEvent
  ;[0 0 0] Set Body Opacity
  (for _array_element (Variables|Don'tEdit!|GetDynamic%20Materials)
    (bind _returnvalue (Rendering|Material|GetScalarParameterValue _array_element "Fade" :!class /Script/Engine.MaterialInstanceDynamic))
    (Rendering|Material|SetScalarParameterValue (Variables|Don'tEdit!|GetDynamic%20Materials) "Fade" (Math|Interpolation|FInterpTo _returnvalue 0.0 (Utilities|Time|GetWorldDeltaSeconds) 1.0) :!class /Script/Engine.MaterialInstanceDynamic)
    (if (Math|Float|NearlyEqual(Float) (Math|Interpolation|FInterpTo _returnvalue 0.0 (Utilities|Time|GetWorldDeltaSeconds) 1.0) 0.0 0.001)
      (Utilities|Time|ClearandInvalidateTimerbyHandle (Variables|Don'tEdit!|GetTimer))
      (bind _as_character (Variables|Don'tEdit!|GetAs%20Character)
        (:then
          (Actor|DestroyActor _as_character))
        (:else)))))

(event Custom|Damage
  (params (Damage :type Float%20%28double-precision%29) (Instigator :type Pawn%20Object%20Reference))
  (bind _returnvalue (Actor|GetComponentbyClass Instigator "/Game/SpellSystemV2/LevelingSystemX/Blueprints/Components/BP_Player_LevelingSystemX.BP_Player_LevelingSystemX_C"))
  ;[0 0 0] Damage
  (if (not (Variables|Don'tEdit!|GetAI%20Dead))
    (CallFunction|NewDamageDealtbyASpecificPlayer Damage Instigator)
    ;[0 0 0] Add Rank Points
    (Utilities|IsValid _returnvalue
      (:Is%20Valid
        (Default|AddRankPoints _returnvalue (Variables|Settings|GetRank%20Points))
        ;[0 0 0] Death
        (if (<= (Variables|Settings|GetCurrent%20Health) 0.0)
          (Variables|Don'tEdit!|SetAI%20Dead true)
          (CallFunction|Death))))))

(event Custom|Death
  (bind _returnvalue (Components|GetOwner))
  ;[0 0 0] Death - Ragdoll / Disable Collision / Spawn EXP
  (Utilities|IsValid _returnvalue
    (:Is%20Valid
      (bind _ascharacter (Utilities|Casting|CastToCharacter _returnvalue))
      (Variables|Don'tEdit!|SetAs%20Character _ascharacter)
      (Variables|Default|SetMesh (Variables|/Script/Engine.Character|GetMesh _ascharacter))
      (for _array_element (Rendering|Material|GetMaterials (Variables|/Script/Engine.Character|GetMesh _ascharacter))
        ;[0 0 0] Create Dynamic Material
        (bind _returnvalue_2 (Rendering|Material|CreateDynamicMaterialInstance _array_element "None" "None" :!class /Script/Engine.KismetMaterialLibrary))
        (bind _returnvalue_3 (Utilities|Array|Add (Variables|Don'tEdit!|GetDynamic%20Materials) _returnvalue_2))
        (Rendering|Material|SetMaterial (Variables|Default|GetMesh) _returnvalue_3 _returnvalue_2))
      (Physics|SetSimulatePhysics (Variables|Default|GetMesh) true)
      (Collision|SetCollisionProfileName (Variables|Default|GetMesh) "Ragdoll" true :!class /Script/Engine.PrimitiveComponent)
      (Collision|SetCollisionResponsetoChannel (Variables|/Script/Engine.Character|GetCapsuleComponent (Variables|Don'tEdit!|GetAs%20Character)) "ECC_Pawn" "ECR_Ignore")
      (Collision|SetCollisionResponsetoChannel (Variables|/Script/Engine.Character|GetCapsuleComponent (Variables|Don'tEdit!|GetAs%20Character)) "ECC_Camera" "ECR_Ignore")
      (Collision|SetCollisionResponsetoChannel (Variables|/Script/Engine.Character|GetCapsuleComponent (Variables|Don'tEdit!|GetAs%20Character)) "ECC_GameTraceChannel1" "ECR_Ignore")
      (Components|Movement|StopMovementImmediately (Variables|/Script/Engine.Character|GetCharacterMovement (Variables|Don'tEdit!|GetAs%20Character)))
      (Utilities|FlowControl|Delay 3.0)
      (CallFunction|SpawnEXP))))

(event Custom|Spawn%20EXP
  (bind _mesh (Variables|Default|GetMesh))
  (bind _returnvalue (Transformation|GetSocketLocation _mesh "pelvis"))
  (bind _returnvalue_2 (+ _returnvalue "0.000000,0.000000,5.000000"))
  ;[0 0 0] Spawn Experience / Add Experience
  (if (Variables|Settings|GetVisualization%20Of%20The%20Experience)
    (for (_array_element _array_index) (Variables|Don'tEdit!|GetPlayers%20Character)
      (if (Variables|Settings|GetPool)
        (bind _returnvalue_3 (Actor|GetActorOfClass "/Game/SpellSystemV2/LevelingSystemX/Blueprints/Actors/BP_PoolManager.BP_PoolManager_C"))
        (Default|GetActorfromPool _returnvalue_3 (Utilities|Struct|MakeS_PoolExperience _returnvalue_2 _array_element (Math|Float|Truncate (* (/ (Utilities|Array|Get(acopy) (Variables|Don'tEdit!|GetDamage%20Done%20By%20Players) _array_index) (Variables|Settings|GetMax%20Health)) (Variables|Settings|GetExperience))) (Variables|Settings|GetEnemy%20Level) (+ (Variables|/Script/Engine.CharacterMovementComponent|GetMaxWalkSpeed (Actor|GetComponentbyClass _array_element "/Script/Engine.CharacterMovementComponent")) 1e+02) (Variables|Settings|GetCollision%20With%20Experience)))
        (else
          (bind _returnvalue_4 (Game|SpawnActorfromClass "/Game/SpellSystemV2/LevelingSystemX/Blueprints/Actors/BP_EXP.BP_EXP_C" (Math|Transform|MakeTransform _returnvalue_2 "0, 0, 0" "1.000000,1.000000,1.000000") "Undefined" 0 (Math|Float|Truncate (* (/ (Utilities|Array|Get(acopy) (Variables|Don'tEdit!|GetDamage%20Done%20By%20Players) _array_index) (Variables|Settings|GetMax%20Health)) (Variables|Settings|GetExperience))) (+ (Variables|/Script/Engine.CharacterMovementComponent|GetMaxWalkSpeed (Actor|GetComponentbyClass _array_element "/Script/Engine.CharacterMovementComponent")) 1e+02) (Variables|Settings|GetEnemy%20Level) (Variables|Settings|GetCollision%20With%20Experience) _array_element))
          (Default|Initialize _returnvalue_4)))
      (if (not (Variables|Settings|GetCollision%20With%20Experience))
        (Networking|SwitchHasAuthority
          (:Authority
            ;;[0 0 0] Add Experience
            (Default|AddExperience-Server (Actor|GetComponentbyClass _array_element "/Game/SpellSystemV2/LevelingSystemX/Blueprints/Components/BP_Player_LevelingSystemX.BP_Player_LevelingSystemX_C") (Math|Float|Truncate (* (/ (Utilities|Array|Get(acopy) (Variables|Don'tEdit!|GetDamage%20Done%20By%20Players) _array_index) (Variables|Settings|GetMax%20Health)) (Variables|Settings|GetExperience))) (Variables|Settings|GetEnemy%20Level))))))
    (CallFunction|OpacityAnimation-Body)
    (else
      (Networking|SwitchHasAuthority
        (:Authority
          (for (_array_element_2 _array_index_2) (Variables|Don'tEdit!|GetPlayers%20Character)
            ;;[0 0 0] Add Experience
            (Default|AddExperience+VisualEffect (Actor|GetComponentbyClass _array_element_2 "/Game/SpellSystemV2/LevelingSystemX/Blueprints/Components/BP_Player_LevelingSystemX.BP_Player_LevelingSystemX_C") (Math|Float|Truncate (* (/ (Utilities|Array|Get(acopy) (Variables|Don'tEdit!|GetDamage%20Done%20By%20Players) _array_index_2) (Variables|Settings|GetMax%20Health)) (Variables|Settings|GetExperience))) (Variables|Settings|GetEnemy%20Level))))
        (:Remote
          _))
      (CallFunction|OpacityAnimation-Body))))

(event Custom|Opacity%20Animation%20-%20Body
  ;[0 0 0] Set Body Opacity
  (bind _returnvalue (Utilities|Time|SetTimerbyEvent (delegate Custom|CustomEvent) 0.016 true))
  (Variables|Don'tEdit!|SetTimer _returnvalue))

(fn NewDamageDealtbyASpecificPlayer
  (params (Damage :type Float%20%28double-precision%29) (Instigator :type Pawn%20Object%20Reference%20%28by%20ref%29))
  ;[0 0 0] Damage Dealt By a Specific Player
  (LocalVariables|SetDamage%20L (Math|Float|Clamp(Float) Damage 0.0 (Variables|Settings|GetCurrent%20Health)))
  (Variables|Settings|SetCurrent%20Health (- (Variables|Settings|GetCurrent%20Health) (LocalVariables|GetDamage%20L)))
  (CallFunction|SetData-Player/Experience Instigator (LocalVariables|GetDamage%20L))
  (return))

(fn SetData-Player/Experience
  (params (Instigator :type Pawn%20Object%20Reference) (Damage :type Float%20%28double-precision%29))
  ;[0 0 0] Set Data
  (if (Utilities|Array|ContainsItem (Variables|Don'tEdit!|GetPlayers%20Character) Instigator)
    (LocalVariables|SetPlayer%20Index%20L (Utilities|Array|FindItem (Variables|Don'tEdit!|GetPlayers%20Character) Instigator))
    (Utilities|Array|SetArrayElem (Variables|Don'tEdit!|GetDamage%20Done%20By%20Players) (LocalVariables|GetPlayer%20Index%20L) (+ (Utilities|Array|Get(acopy) (Variables|Don'tEdit!|GetDamage%20Done%20By%20Players) (LocalVariables|GetPlayer%20Index%20L)) Damage))
    (else
      (Utilities|Array|Add (Variables|Don'tEdit!|GetPlayers%20Character) Instigator)
      (Utilities|Array|Add (Variables|Don'tEdit!|GetDamage%20Done%20By%20Players) Damage))))