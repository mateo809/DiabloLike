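; Base damage spell actor that plays a looping Niagara effect until its sphere overlaps or hits another actor.
; Contacts with its owner or actors sharing its instigator are ignored; others stop the loop and disable collision.
; The server applies the damage, while non-dedicated instances spawn the hit effect.
; The actor destroys itself when that effect finishes, a path that never runs on dedicated servers.
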(event OnComponentBeginOverlap(Sphere)
  (params (OverlappedComponent :type Primitive%20Component%20Object%20Reference) (OtherActor :type Actor%20Object%20Reference) (OtherComp :type Primitive%20Component%20Object%20Reference) (OtherBodyIndex :type Integer) (bFromSweep :type Boolean) (SweepResult :type Hit%20Result%20Structure%20%28by%20ref%29))
  ;[0 0 0] Hit
  (Variables|Default|SetHitActor OtherActor)
  (if (!= (Components|GetOwner) (Variables|Default|GetHitActor))
    (if (not (== (Game|GetInstigator (Variables|Default|GetHitActor)) (Game|GetInstigator)))
      (Components|Activation|Deactivate (Variables|Default|GetNiagara))
      (Collision|SetCollisionEnabled (Variables|Default|GetSphere) "NoCollision")
      (if (Networking|IsDedicatedServer)
        _
        (else
          (bind _returnvalue (Niagara|SpawnSystematLocation (Variables|Settings|GetSystem%20-%20Hit) (Transformation|GetActorLocation)))
          (EventDispatchers|BindEventtoOnSystemFinished _returnvalue (delegate Custom|CustomEvent))))
      (if (or (Networking|IsServer) (Networking|IsDedicatedServer))
        (Game|Damage|ApplyDamage (Variables|Default|GetHitActor) (Variables|Default|GetValue) 0 (Variables|Default|GetInstigator))))))

(event OnComponentHit(Sphere)
  (params (HitComponent :type Primitive%20Component%20Object%20Reference) (OtherActor :type Actor%20Object%20Reference) (OtherComp :type Primitive%20Component%20Object%20Reference) (NormalImpulse :type Vector :default "0, 0, 0") (Hit :type Hit%20Result%20Structure%20%28by%20ref%29))
  ;[0 0 0] Hit
  (Variables|Default|SetHitActor OtherActor)
  (if (!= (Components|GetOwner) (Variables|Default|GetHitActor))
    (if (not (== (Game|GetInstigator (Variables|Default|GetHitActor)) (Game|GetInstigator)))
      (Components|Activation|Deactivate (Variables|Default|GetNiagara))
      (Collision|SetCollisionEnabled (Variables|Default|GetSphere) "NoCollision")
      (if (Networking|IsDedicatedServer)
        _
        (else
          (bind _returnvalue (Niagara|SpawnSystematLocation (Variables|Settings|GetSystem%20-%20Hit) (Transformation|GetActorLocation)))
          (EventDispatchers|BindEventtoOnSystemFinished _returnvalue (delegate Custom|CustomEvent))))
      (if (or (Networking|IsServer) (Networking|IsDedicatedServer))
        (Game|Damage|ApplyDamage (Variables|Default|GetHitActor) (Variables|Default|GetValue) 0 (Variables|Default|GetInstigator))))))

(event Custom|CustomEvent
  (params (PSystem :type Niagara%20Component%20Object%20Reference))
  ;[0 0 0] Hit
  (Actor|DestroyActor))

(event EventBeginPlay
  ;[0 0 0] Begin Play
  (Class|NiagaraComponent|SetAsset (Variables|Default|GetNiagara) (Variables|Settings|GetSystem%20-%20Loop) true))

(fn ConstructionScript)