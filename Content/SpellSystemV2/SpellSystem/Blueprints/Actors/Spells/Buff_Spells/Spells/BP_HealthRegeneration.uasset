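; A buff spell actor that restores health to the character that cast it.
; On begin play, the server finds the SpellSystem component on its instigator and increases health by the spell's Value.
; The actor destroys itself when its Niagara effect finishes.
; Despite the regeneration name, the graph applies the health increase in a single call rather than over time.
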(event Custom|CustomEvent_1
  (params (PSystem :type Niagara%20Component%20Object%20Reference))
  ;[0 0 0] Begin Play
  (Actor|DestroyActor))

(event EventBeginPlay
  ;[0 0 0] Begin Play
  (|CallParentFunction)
  (EventDispatchers|BindEventtoOnSystemFinished (Variables|Default|GetNiagara) (delegate Custom|CustomEvent_1))
  (if (Networking|IsServer)
    (Default|IncreaseHealth (Actor|GetComponentbyClass (Game|GetInstigator) "/Game/SpellSystemV2/SpellSystem/Blueprints/SpellSystem_Component.SpellSystem_Component_C") (Variables|Default|GetValue))))

(fn ConstructionScript
  (|CallParentFunction))